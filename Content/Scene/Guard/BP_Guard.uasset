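; BP_Guard is a guard actor that confronts the player when it overlaps an illegal puzzle item.
; On begin overlap, it filters for actors implementing I_Illegal, casts to BP_Puzzle_Item and checks IsLegal.
; For an illegal item, it shows an accusation naming the item through the FirstPersonCharacter's message display, then calls the illegal event dispatcher.
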(event `self.ReceiveActorBeginOverlap`
  (params (OtherActor :type "Actor Object Reference"))
  ;[1 1 1] Send Event if enters illegal Item's collider
  (bind _output_get (set `self.Other Actor` OtherActor))
  (if (`KismetSystemLibrary.DoesImplementInterface` _output_get "/Game/Scene/Interactions/Puzzle/I_Illegal.I_Illegal_C")
    (bind _asbp_puzzle_item (cast `/Game/Scene/Interactions/Puzzle/BP_Puzzle_Item` (`self.Other Actor`)))
    (bind _islegalbool (`/Game/Scene/Interactions/Puzzle/BP_Puzzle_Item.isLegal` _asbp_puzzle_item))
    (if (not _islegalbool)
      (bind _asfirst_person_character (cast `/Game/Default_FirstPersonBP/Blueprints/FirstPersonCharacter` (`GameplayStatics.GetPlayerCharacter` 0)))
      (bind _unlockitemstructureinfo_name (break `/Game/Scene/Interactions/Puzzle/PuzzleStructure` (`/Game/Scene/Interactions/Puzzle/BP_Puzzle_Item.UnlockItemStructureInfo` _asbp_puzzle_item)))
      (`/Game/Default_FirstPersonBP/Blueprints/FirstPersonCharacter.DisplayingMessage` _asfirst_person_character (`KismetStringLibrary.Concat_StrStr` "Hey you ! Is this a " _unlockitemstructureinfo_name " ? This is illegal ! Explain yourself !") (make `Color` 0 0 255 255))
      (`self.IllegalEventDispatcher`))))

(fn `UserConstructionScript`)