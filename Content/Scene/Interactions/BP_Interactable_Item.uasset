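; Base Blueprint for interactable items that shows an interaction UI when the player interacts with one.
; Interacting creates a W_Interaction widget bound to the item, adds it to the viewport and activates it.
; It casts itself to the child classes to label the action "Pick" for pickable items or "Solve" for puzzle items.
; GetExamineMessage supplies the examine text from the item's structure description.
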(event `/Game/Widgets_UI/Interaction_UI/I_Interactable.Interacting`
  (bind _display_interact_ui (`self.Display Interact UI`))
  ;[1 1 1] Display Interaction Widget when interacting with interactable object
  (bind _returnvalue (`|CreateWidget` "/Game/Widgets_UI/Interaction_UI/W_Interaction.W_Interaction_C" null self))
  (set `self.Display Interact UI` _returnvalue)
  (if (not (`Widget.IsInViewport` _display_interact_ui))
    (`UserWidget.AddToViewport` (`self.Display Interact UI`) 0)
    (`/Game/Widgets_UI/Interaction_UI/W_Interaction.Activate Interaction UI` _display_interact_ui)
    ;[1 1 1] Will change (Action) text to Pick or Solve depending on child
    (cast `/Game/Scene/Interactions/Pickable/BP_Pickable_Item` self
      (:`then`
        (`self.updateActionText` "Pick"))
      (:`CastFailed`
        (cast `/Game/Scene/Interactions/Puzzle/BP_Puzzle_Item` self)
        (`self.updateActionText` "Solve")))))

(fn `getExamineMessage`
  (returns (parMessage :type String))
  (bind (_itemstructuresinfo_name _itemstructuresinfo_icon _itemstructuresinfo_description) (break `/Game/Scene/Interactions/Pickable/ItemStructures` (`self.ItemStructuresInfo`)))
  ;[1 1 1] Returns the message to display when examinating items
  (return _itemstructuresinfo_description))

(fn `updateActionText`
  (params (parText :type String))
  ;[1 1 1] Change (Action) text with parText
  (`TextBlock.SetText` (`/Game/Widgets_UI/Interaction_UI/W_Interaction.ActionText` (`self.Display Interact UI`)) (`KismetTextLibrary.Conv_StringToText` parText)))

(fn `UserConstructionScript`)