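; BP_Pickable_Item is a pickable world item that can be collected into the player's inventory.
; Its construction script fills an item info struct with a default name and description.
; The Pickitem event casts the player character to FirstPersonCharacter, adds that struct through its inventory widget, prints debug messages and destroys the actor.
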(event `Pick item`
  (`KismetSystemLibrary.PrintString` "1- Picking up item")
  (bind _asfirst_person_character (cast `/Game/Default_FirstPersonBP/Blueprints/FirstPersonCharacter` (`GameplayStatics.GetPlayerCharacter` 0)))
  (`KismetSystemLibrary.PrintString` "Adding to inventory")
  (`/Game/Widgets_UI/Inventory_UI/W_Inventory.Add Item to Inventory` (`/Game/Default_FirstPersonBP/Blueprints/FirstPersonCharacter.Inventory_Widget` _asfirst_person_character) (`self.ItemStructuresInfo`))
  (`self.K2_DestroyActor`))

(fn `UserConstructionScript`
  (`parent.UserConstructionScript`)
  (set `self.ItemStructuresInfo` (make `/Game/Scene/Interactions/Pickable/ItemStructures` "PickableItem" null "This is a pickable item")))