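; Cell door puzzle interactable, a child Blueprint that leads to the final code entry screen.
; The construction script fills the inherited unlock info with the door's name, hint text and the "Final Key" item.
; When the parent's SolvingPuzzle check succeeds, it adds the player character's FinalCodeUI to the viewport and activates it, unless already shown.
; IsLegal calls the parent but always returns true.
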(fn `isLegal`
  (returns (isLegalBool :type Boolean))
  (`parent.isLegal`)
  (return true))

(fn `SolvingPuzzle`
  (params (UnlockItemName :type String))
  (returns (isRightItem :type Boolean))
  (bind _isrightitem (`parent.SolvingPuzzle` UnlockItemName))
  (if _isrightitem
    (bind _asfirst_person_character (cast `/Game/Default_FirstPersonBP/Blueprints/FirstPersonCharacter` (`GameplayStatics.GetPlayerCharacter` 0)))
    (bind _finalcodeui (`/Game/Default_FirstPersonBP/Blueprints/FirstPersonCharacter.FinalCodeUI` _asfirst_person_character))
    (if (not (`Widget.IsInViewport` _finalcodeui))
      (`UserWidget.AddToViewport` _finalcodeui 0)
      (`/Game/Widgets_UI/FinalCode_UI/W_FinalCode.ActivateFinalCodeUI` _finalcodeui))))

(fn `UserConstructionScript`
  (`parent.UserConstructionScript`)
  (set `self.UnlockItemStructureInfo` (make `/Game/Scene/Interactions/Puzzle/PuzzleStructure` "Cell door" "It seems like I could put some kind of square in here" "Final Key")))