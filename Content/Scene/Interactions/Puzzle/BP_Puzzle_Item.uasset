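; Puzzle interactable that checks whether a given item, meant to be the one the player holds, is the right one to solve it.
; The construction script fills an unlock-item struct with placeholder puzzle data, whose description serves as the examine message.
; SolvingPuzzle compares names, shows success or failure text through FirstPersonCharacter, and fires a wasting-time dispatcher on a mismatch.
; The SolvePuzzle event is an empty stub.
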(event `/Game/Scene/Interactions/Puzzle/I_Solve.Solve Puzzle`
  (params (UnlockItemName :type String)))

(fn `getExamineMessage`
  (returns (parMessage :type String))
  (bind (_unlockitemstructureinfo_name _unlockitemstructureinfo_description) (break `/Game/Scene/Interactions/Puzzle/PuzzleStructure` (`self.UnlockItemStructureInfo`)))
  (`parent.getExamineMessage`)
  (return _unlockitemstructureinfo_description))

(fn `isLegal`
  (returns (isLegalBool :type Boolean))
  (return (`self.isLegalBool`)))

(fn `SolvingPuzzle`
  (params (UnlockItemName :type String))
  (returns (isRightItem :type Boolean))
  (bind (_unlockitemstructureinfo_name _unlockitemstructureinfo_description _unlockitemstructureinfo_unlockitemname) (break `/Game/Scene/Interactions/Puzzle/PuzzleStructure` (`self.UnlockItemStructureInfo`)))
  (bind _returnvalue (`KismetStringLibrary.EqualEqual_StrStr` UnlockItemName _unlockitemstructureinfo_unlockitemname))
  ;[1 1 1] Player's Holding item == Puzzle's Unlock item
  (bind _asfirst_person_character (cast `/Game/Default_FirstPersonBP/Blueprints/FirstPersonCharacter` (`GameplayStatics.GetPlayerCharacter` 0)))
  (if _returnvalue
    (`/Game/Default_FirstPersonBP/Blueprints/FirstPersonCharacter.DisplayingMessage` _asfirst_person_character (`KismetStringLibrary.Concat_StrStr` "Yes ! " UnlockItemName " was the right item to solve this " _unlockitemstructureinfo_name) (make `Color` 0 255 0 255))
    (return _returnvalue)
    (else
      (`/Game/Default_FirstPersonBP/Blueprints/FirstPersonCharacter.DisplayingMessage` _asfirst_person_character (`KismetStringLibrary.Concat_StrStr` "You are wasting time with this " UnlockItemName " ! This is not the right item to solve this " _unlockitemstructureinfo_name) (make `Color` 102 178 255 255))
      (`self.WastingTimeEventDispatcher`))))

(fn `UserConstructionScript`
  (`parent.UserConstructionScript`)
  (set `self.UnlockItemStructureInfo` (make `/Game/Scene/Interactions/Puzzle/PuzzleStructure` "PuzzleItem" "This is a puzzle you have to solve" "PuzzleItem")))