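; Digital chest puzzle interactable that swings open when SolvePuzzle is called and supplies its name and hint text.
; OpenFront toggles IsFrontClosed, playing or reversing a timeline that yaws Root between 0 and 90 degrees.
; IsLegal returns true only while the front is closed.
; The keypad code path is unfinished: the UI_Pad binding is unconnected, CodeEnteredEvent is empty and CheckCode compares against CorrectCode without acting.
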(event `self.ReceiveBeginPlay`)

(event `CodeEnteredEvent`
  (params (Code :type String) (Pad :type "/Game/Scene/Interactions/Puzzle/DigitalChest/UI_Pad Object Reference")))

(event `Open Front`
  (if (`self.IsFrontClosed`)
    (set `self.IsFrontClosed` false)
    (bind (_direction _alpha) (`Timeline|TL_OpenFront` :!label _label)
      (:`Update`
        (`SceneComponent.K2_SetRelativeRotation` (`self.root`) (`KismetMathLibrary.MakeRotator` 0.0 0.0 (`KismetMathLibrary.Lerp` 0.0 90.0 _alpha)) false false)))
    (else
      (set `self.IsFrontClosed` true)
      (goto _label :!via `Reverse`))))

(event `/Game/Scene/Interactions/Puzzle/I_Solve.Solve Puzzle`
  (params (UnlockItemName :type String))
  (`KismetSystemLibrary.PrintString` "Try to open chest")
  (`self.Open Front`))

(fn `CheckCode`
  (params (CodeEntered :type String) (UI_Pad :type "/Game/Scene/Interactions/Puzzle/DigitalChest/UI_Pad Object Reference"))
  (if (`KismetStringLibrary.EqualEqual_StrStr` CodeEntered (`self.CorrectCode`))
    _))

(fn `isLegal`
  (returns (isLegalBool :type Boolean))
  (`parent.isLegal`)
  (return (`self.IsFrontClosed`)))

(fn `UserConstructionScript`
  (`parent.UserConstructionScript`)
  (set `self.ItemStructuresInfo` (make `/Game/Scene/Interactions/Pickable/ItemStructures` "Digital Chest" null "This is a digital chest, how will you open it ?")))