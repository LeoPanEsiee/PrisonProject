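; BP_Clock is the game's countdown clock, ending the game with a fail screen and pause at 60 minutes.
; Tick uses a Delay to add a minute every five seconds, then updates the W_Time text, turns it red late in the hour and rotates the minute hand.
; Dispatchers from BP_Guard and BP_Puzzle_Item add penalty minutes for illegal items or wrong puzzle items; a TODO notes immediate display updates are still pending.
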(event `self.ReceiveBeginPlay`
  ;[1 1 1] Adding Time UI to Scene
  (bind _returnvalue (`|CreateWidget` "/Game/Time_UI/W_Time.W_Time_C"))
  (bind _output_get (set `self.Timer_UI` _returnvalue))
  (`UserWidget.AddToViewport` _output_get 0)
  ;[1 1 1] Guard saw an illegal item
  (bind _returnvalue_2 (`GameplayStatics.GetActorOfClass` "/Game/Scene_Elements/Guard/BP_Guard.BP_Guard_C"))
  (add `/Game/Scene_Elements/Guard/BP_Guard.IllegalEventDispatcher` _returnvalue_2 (delegate `IllegalPenality`))
  ;[1 1 1] The player used the wrong item on a puzzle
  (bind _outactors (`GameplayStatics.GetAllActorsOfClass` "/Game/Scene_Elements/Interactions/Puzzle/BP_Puzzle_Item.BP_Puzzle_Item_C"))
  (add `/Game/Scene_Elements/Interactions/Puzzle/BP_Puzzle_Item.WastingTimeEventDispatcher` _outactors (delegate `WasteTimePenalty`)))

(event `IllegalPenality`
  ;[1 1 1] Guard saw an illegal item
  (set `self.CurrentMinute` (+ (`self.CurrentMinute`) 5))
  (`self.UpdateTime`))

(event `WasteTimePenalty`
  ;[1 1 1] The player used the wrong item on a puzzle
  (set `self.CurrentMinute` (+ (`self.CurrentMinute`) 1))
  (`self.UpdateTime`))

(event `UpdateTime`
  (bind _minuteroot (`self.MinuteRoot`))
  (bind (_relativerotation_roll _relativerotation_pitch _relativerotation_yaw) (`KismetMathLibrary.BreakRotator` (`SceneComponent.RelativeRotation` _minuteroot)))
  (bind _minutestext (`/Game/Time_UI/W_Time.MinutesText` (`self.Timer_UI`)))
  ;[1 1 1] TODO : Update immediatly the time when a penalty is given
  (`KismetSystemLibrary.PrintString` "Updating time")
  (`KismetSystemLibrary.PrintString` (`KismetStringLibrary.Conv_IntToString` (`self.CurrentMinute`)))
  ;[1 1 1] UI Text From 0 to 9 minutes
  (if (< (stale `self.ReceiveTick` _result) 10) :!label _label
    (`TextBlock.SetText` (`/Game/Time_UI/W_Time.MinutesText` (`self.Timer_UI`)) (`KismetTextLibrary.Conv_StringToText` (`KismetStringLibrary.Concat_StrStr` "0" (`KismetStringLibrary.Conv_IntToString` (stale `self.ReceiveTick` _result)))))
    (else
      ;[1 0.1356 0.2333] If Only 15 minutes left, paint in red
      (if (>= (`self.CurrentMinute`) 45)
        (`TextBlock.SetColorAndOpacity` _minutestext (make `SlateColor` (struct :`R` 1.0 :`A` 1.0)))
        (`TextBlock.SetColorAndOpacity` (`/Game/Time_UI/W_Time.HourText` (`self.Timer_UI`)) (make `SlateColor` (struct :`R` 1.0 :`A` 1.0))))
      (`TextBlock.SetText` _minutestext (`KismetTextLibrary.Conv_IntToText` (stale `self.ReceiveTick` _result)))))
  ;[1 1 1] Moving the minute Hand
  (`SceneComponent.K2_SetRelativeRotation` _minuteroot (`KismetMathLibrary.MakeRotator` _relativerotation_roll _relativerotation_pitch (`KismetMathLibrary.Conv_IntToDouble` (* (`self.CurrentMinute`) 6))) false false)
  ;[1 1 1] Lose the game if timer is after 60 minutes
  (if (>= (`self.CurrentMinute`) 60)
    (`self.LoseGame`)))

(event `self.ReceiveTick`
  (params (DeltaSeconds :type "Float (single-precision)"))
  (`KismetSystemLibrary.Delay` 5.0)
  (bind _result (`/Engine/EditorBlueprintResources/StandardMacros.IncrementInt` (`self.CurrentMinute`))
    (:`  `
      (goto _label))))

(fn `LoseGame`
  (bind _returnvalue (`GameplayStatics.GetPlayerController` 0))
  (bind _returnvalue_2 (`|CreateWidget` "/Game/Fail_Game/Widget_Fail.Widget_Fail_C"))
  (`UserWidget.AddToViewport` _returnvalue_2 0)
  (`Widget.SetVisibility` _returnvalue_2 "Visible")
  (`WidgetBlueprintLibrary.SetInputMode_GameAndUIEx` _returnvalue null)
  (set `PlayerController.bShowMouseCursor` true _returnvalue)
  (`GameplayStatics.SetGamePaused` true)
  (`self.DisableInput` (`GameplayStatics.GetPlayerCharacter` 0) (`GameplayStatics.GetPlayerController` 0)))

(fn `UserConstructionScript`)