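; BP_Key_old is a key interactable that shows an interaction UI when interacted with.
; Its Interacting event creates a new W_Interaction widget with itself as ObjectToTake and stores it in DisplayInteractUI.
; It deactivates the widget if already in the viewport, otherwise adds and activates it.
; Because the widget is recreated before that check, each call tests the new instance, not the previous one.
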(event `/Game/Scene_Elements/Interactions/I_Interactable.Interacting`
  (bind _display_interact_ui (`self.Display Interact UI`))
  (bind _returnvalue (`|CreateWidget` "/Game/Scene_Elements/Interactions/W_Interaction.W_Interaction_C" null self))
  (set `self.Display Interact UI` _returnvalue)
  (if (`Widget.IsInViewport` _display_interact_ui)
    (`/Game/Scene_Elements/Interactions/W_Interaction.Deactivate Interaction UI` (`self.Display Interact UI`))
    (else
      (`UserWidget.AddToViewport` (`self.Display Interact UI`) 0)
      (`/Game/Scene_Elements/Interactions/W_Interaction.Activate Interaction UI` _display_interact_ui))))

(fn `UserConstructionScript`)