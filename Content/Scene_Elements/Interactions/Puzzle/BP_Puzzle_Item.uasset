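; Base puzzle interactable that defines what item solves it and what examine text it shows.
; The construction script fills the unlock item struct with placeholder puzzle text and names, and the examine message returns that description.
; SolvingPuzzle checks a given item name, meant as the player's held item, against the unlock name.
; SolvePuzzle is an empty event, and IsLegal exposes a stored flag.
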(event `/Game/Scene_Elements/Interactions/Puzzle/I_Solve.Solve Puzzle`
  (params (UnlockItemName :type String)))

(fn `getExamineMessage`
  (returns (parMessage :type String))
  (bind (_unlockitemstructureinfo_name _unlockitemstructureinfo_description) (break `/Game/Scene_Elements/Interactions/Puzzle/PuzzleStructure` (`self.UnlockItemStructureInfo`)))
  (`parent.getExamineMessage`)
  (return _unlockitemstructureinfo_description))

(fn `isLegal`
  (returns (isLegalBool :type Boolean))
  (return (`self.isLegalBool`)))

(fn `SolvingPuzzle`
  (params (UnlockItemName :type String))
  (returns (isRightItem :type Boolean))
  (bind (_unlockitemstructureinfo_name _unlockitemstructureinfo_description _unlockitemstructureinfo_unlockitemname) (break `/Game/Scene_Elements/Interactions/Puzzle/PuzzleStructure` (`self.UnlockItemStructureInfo`)))
  ;[1 1 1] Player's Holding item == Puzzle's Unlock item
  (return (`KismetStringLibrary.EqualEqual_StrStr` UnlockItemName _unlockitemstructureinfo_unlockitemname)))

(fn `UserConstructionScript`
  (`parent.UserConstructionScript`)
  (set `self.UnlockItemStructureInfo` (make `/Game/Scene_Elements/Interactions/Puzzle/PuzzleStructure` "PuzzleItem" "This is a puzzle you have to solve" "PuzzleItem")))